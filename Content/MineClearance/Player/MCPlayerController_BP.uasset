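; Player controller for the minesweeper game, managing cursor and input setup, HUD, music, pause state and game end.
; BeginPlay configures the mouse by the GameInstance's FirstPlayer flag, creates both widgets and copies the mine count into FlagNum.
; Escape flips pause via FlipFlops that toggle a one-second timer and input mode, without pausing the world.
; Exceeding the time limit sets GameResult; Tick polls it to show the result screen once.
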(event `self.ReceiveBeginPlay`
  (bind _returnvalue (`GameplayStatics.GetPlayerController` 0))
  (bind _returnvalue_2 (`GameplayStatics.GetPlayerController` 0))
  ;[1 1 1] 开始
  (`|ExecutionSequence`
    (:`then_0`
      (bind _asmcgame_instance_bp (cast `/Game/MineClearance/Player/MCGameInstance_BP` (`GameplayStatics.GetGameInstance`)))
      (set `self.GameInstance` _asmcgame_instance_bp)
      (if (`MCGameInstance.bFirstPlayer` _asmcgame_instance_bp)
        (set `PlayerController.bShowMouseCursor` false _returnvalue_2)
        (set `PlayerController.bEnableClickEvents` false _returnvalue_2)
        (set `PlayerController.bEnableTouchEvents` false _returnvalue_2)
        (else
          (set `PlayerController.bShowMouseCursor` true _returnvalue_2)
          (set `PlayerController.bEnableClickEvents` true _returnvalue_2)
          (set `PlayerController.bEnableTouchEvents` true _returnvalue_2))))
    (:`then_1`
      (`self.StopGame_Switch`))
    (:`then_2`
      (bind _returnvalue_3 (`|CreateWidget` "/Game/MineClearance/UI/InGame.InGame_C" _returnvalue))
      (bind _output_get (set `self.InGameUI` _returnvalue_3))
      (`UserWidget.AddToViewport` _output_get 0))
    (:`then_3`
      (bind _returnvalue_4 (`|CreateWidget` "/Game/MineClearance/UI/GameResult.GameResult_C" _returnvalue))
      (set `self.ResultUI` _returnvalue_4))
    (:`then_4`
      (`GameplayStatics.PlaySound2D` "/Game/MineClearance/Audio/BGM.BGM" 1.0 1.0 0.0 null null))
    (:`then_5`
      (bind _asmcgame_instance_bp_2 (cast `/Game/MineClearance/Player/MCGameInstance_BP` (`GameplayStatics.GetGameInstance`)))
      (set `self.FlagNum` (`MCGameInstance.MinesNumber` _asmcgame_instance_bp_2)))))

(event `InputAction|Escape`
  (params (Key :type "Key Structure"))
  ;[1 1 1] 返回按键
  (:`Pressed`
    (`self.StopGame_Switch`)))

(event `StopGame_Switch`
  (bind _returnvalue (`GameplayStatics.GetPlayerController` 0))
  ;[1 1 1] 切换游戏暂停状态
  (bind _isa (`/Engine/EditorBlueprintResources/StandardMacros.FlipFlop`)
    (:`A`
      (bind _returnvalue_2 (`KismetSystemLibrary.K2_SetTimerDelegate` (delegate `TimerEvent`) 1.0 true))
      (set `self.Timer` _returnvalue_2)
      (if (`MCGameInstance.bFirstPlayer` (`self.GameInstance`))
        (set `PlayerController.bShowMouseCursor` false _returnvalue)))
    (:`B`
      (`KismetSystemLibrary.K2_ClearAndInvalidateTimerHandle` (`self.Timer`))
      (set `PlayerController.bShowMouseCursor` true _returnvalue)))
  (`self.SwitchGamePause`)
  (set `self.Stop` (not _isa)))

(event `TimerEvent`
  ;[1 1 1] 切换游戏暂停状态
  (bind _result (`/Engine/EditorBlueprintResources/StandardMacros.IncrementInt` (`self.Time`))
    (:`  `
      (if (> _result (`self.MaxTimeLimit`))
        (set `self.GameResult` 2)))))

(event `SwitchGamePause`
  (bind _returnvalue (`GameplayStatics.GetPlayerController` 0))
  (bind _ingameui (`self.InGameUI`))
  ;[1 1 1] 切换游戏暂停状态
  (`/Engine/EditorBlueprintResources/StandardMacros.FlipFlop`
    (:`A`
      (if (`MCGameInstance.bFirstPlayer` (`self.GameInstance`))
        (`WidgetBlueprintLibrary.SetInputMode_GameOnly` _returnvalue)
        (else
          (`WidgetBlueprintLibrary.SetInputMode_GameAndUIEx` _returnvalue _ingameui))))
    (:`B`
      (`WidgetBlueprintLibrary.SetInputMode_UIOnlyEx` _returnvalue _ingameui))))

(event `self.ReceiveTick`
  (params (DeltaSeconds :type "Float (single-precision)"))
  (bind _returnvalue (`GameplayStatics.GetPlayerController` 0))
  ;[1 1 1] 胜利检测
  (if (> (`self.GameResult`) 0)
    (`/Engine/EditorBlueprintResources/StandardMacros.DoOnce` false
      (:`Completed`
        (`self.StopGame_Switch`)
        (`Widget.RemoveFromParent` (`self.InGameUI`))
        (`UserWidget.AddToViewport` (`self.ResultUI`) 0)
        (`WidgetBlueprintLibrary.SetInputMode_UIOnlyEx` _returnvalue null)
        (set `PlayerController.bShowMouseCursor` true _returnvalue)))))

(fn `UserConstructionScript`)