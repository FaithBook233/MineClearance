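; MCPawn_BP is the player pawn in a Minesweeper-style game, handling right-click flagging of grid blocks.
; On right mouse press, it traces on the Camera channel from the pawn's location along the deprojected mouse direction.
; A hit MCBlock toggles its sign, its owning grid runs GameWin, and the grid's current flag count is copied to MCPlayerController_BP.
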(event `InputAction|Mouse_R`
  (params (Key :type "Key Structure"))
  (bind _returnvalue (`self.K2_GetActorLocation`))
  ;[1 1 1] 鼠标右键
  (:`Pressed`
    (bind (_outhit _returnvalue_2) (`KismetSystemLibrary.LineTraceSingle` _returnvalue (+ _returnvalue (* (`.WorldDirection` (`PlayerController.DeprojectMousePositionToWorld` (`GameplayStatics.GetPlayerController` 0))) (`self.RayLength`))) "TraceTypeQuery2"))
    (if _returnvalue_2
      (bind _asmcblock (cast `MCBlock` (`.HitActor` (`GameplayStatics.BreakHitResult` _outhit))))
      (`MCBlock.SwitchSign` _asmcblock)
      (bind _owninggrid (`MCBlock.OwningGrid` _asmcblock))
      (`MCBlockGrid.GameWin` _owninggrid)
      (bind _asmcplayer_controller_bp (cast `/Game/MineClearance/Player/MCPlayerController_BP` (`GameplayStatics.GetPlayerController` 0)))
      (set `/Game/MineClearance/Player/MCPlayerController_BP.FlagNum` (`MCBlockGrid.CurrentFlagNum` _owninggrid) _asmcplayer_controller_bp))))

(fn `UserConstructionScript`)